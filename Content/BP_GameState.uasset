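; Game state Blueprint that tracks player controllers, assigns player IDs and relays score updates.
; AddPC stores each controller and starts a one-second, non-looping timer, after which every controlled pawn receives its array index as its ID through an interface message.
; UpdatePlayerScore sends the given score and ID to all controlled pawns through the same message-based approach.
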(event Custom|UpdatePlayerScore
  (params (PlayerScore :type Integer) (ID :type Integer))
  (for _array_element (Variables|Default|GetPlayerControllers)
    (Class|BPIPlayer|IUpdatePlayerScore(Message) (Pawn|GetControlledPawn _array_element) PlayerScore ID)))

(event Custom|AddPC
  (params (NewItem :type Player%20Controller%20Object%20Reference%20%28by%20ref%29))
  (Utilities|Array|Add (Variables|Default|GetPlayerControllers) NewItem)
  (CallFunction|SetIDTimer)
  (Development|PrintString (Utilities|String|Append "Added PC: " (Utilities|GetDisplayName NewItem)) true true "(R=0.000000,G=0.660000,B=1.000000,A=1.000000)" 1e+01))

(event Custom|SetIDTimer
  (bind _returnvalue (Utilities|Time|SetTimerbyEvent (delegate Custom|SetIDTick) 1.0))
  (Variables|Default|SetIDTimerHandle _returnvalue))

(event Custom|SetIDTick
  (Variables|Default|SetIDIndex 0)
  (for (_array_element _array_index) (Variables|Default|GetPlayerControllers)
    (Class|BPIPlayer|ISetID(Message) (Pawn|GetControlledPawn _array_element) _array_index)))

(event EventBeginPlay)

(fn ConstructionScript)